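; Door1 is a key-locked door actor that slides along Z when the third-person character enters its Box trigger carrying a key.
; Entering with a key decrements the character's KeyAmmount and plays the DoorDown timeline, whose Slide track sets the actor's relative Z, with X and Y from the Door1 component.
; Entering without a key and any end overlap both hide the TextRender; nothing here shows it.
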(event OnComponentBeginOverlap(Box)
  (params (OverlappedComponent :type Primitive%20Component%20Object%20Reference) (OtherActor :type Actor%20Object%20Reference) (OtherComp :type Primitive%20Component%20Object%20Reference) (OtherBodyIndex :type Integer) (bFromSweep :type Boolean) (SweepResult :type Hit%20Result%20Structure%20%28by%20ref%29))
  (bind _door1 (Variables|Default|Getdoor1))
  (bind _relativelocation (Variables|/Script/Engine.SceneComponent|GetRelativeLocation _door1))
  (bind _asbp_third_person_character (Utilities|Casting|CastToBP_ThirdPersonCharacter OtherActor))
  (if (>= (Variables|/Game/ThirdPerson/Blueprints/BP_ThirdPersonCharacter.BP_ThirdPersonCharacter_C|GetKeyAmmount _asbp_third_person_character) 1)
    (Variables|/Game/ThirdPerson/Blueprints/BP_ThirdPersonCharacter.BP_ThirdPersonCharacter_C|SetKeyAmmount _asbp_third_person_character (- (Variables|/Game/ThirdPerson/Blueprints/BP_ThirdPersonCharacter.BP_ThirdPersonCharacter_C|GetKeyAmmount _asbp_third_person_character) 1))
    (bind _slide (Timeline|Door%20down Play)
      (:Update
        (Transformation|SetActorRelativeLocation (Math|Vector|MakeVector (.x _relativelocation) (.y _relativelocation) _slide))))
    (else
      (Rendering|SetVisibility (Variables|Default|GetTextRender) false false))))

(event OnComponentEndOverlap(Box)
  (params (OverlappedComponent :type Primitive%20Component%20Object%20Reference) (OtherActor :type Actor%20Object%20Reference) (OtherComp :type Primitive%20Component%20Object%20Reference) (OtherBodyIndex :type Integer))
  (Rendering|SetVisibility (Variables|Default|GetTextRender) false false))

(event EventBeginPlay)

(event Collision|EventActorBeginOverlap
  (params (OtherActor :type Actor%20Object%20Reference)))

(event EventTick
  (params (DeltaSeconds :type Float%20%28single-precision%29)))

(fn ConstructionScript)